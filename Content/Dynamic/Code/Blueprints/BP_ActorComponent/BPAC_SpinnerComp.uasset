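; Static mesh component on the first-person character that shows an inventory or audio item as a 3D inspection view.
; StartSpin takes the mesh and spin scale from the item's data asset, reveals the component and swaps the default Enhanced Input mapping context for the item-spinner one.
; EndSpin hides and clears the mesh, resets its rotation and restores default input.
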(event `self.ReceiveBeginPlay`
  ;[1 1 1] Setting Up Controller Reference
  (bind _asbp_first_person_character (cast `/Game/Dynamic/Code/Blueprints/Character/BP_FirstPersonCharacter` (`self.GetOwner`)))
  (bind _output_get (set `self.Charater Ref` _asbp_first_person_character))
  (bind _asbp_first_person_player_controller (cast `/Game/Dynamic/Code/Blueprints/Character/BP_FirstPersonPlayerController` (`Pawn.GetController` _output_get)))
  (set `self.Controller Ref` _asbp_first_person_player_controller))

(event `StartSpin`
  (params (PDA_Ref :type "/Game/Dynamic/Code/Blueprints/BP_Pickups/PDA_Parent_Item Object Reference"))
  (bind _returnvalue (pcsubsystem `EnhancedInputLocalPlayerSubsystem` (`self.Controller Ref`)))
  ;[1 1 1] Getting the item type and then passing in that items static mesh and selected scale.
  (bind _aspda_inventory_item (cast `/Game/Dynamic/Code/Blueprints/BP_Pickups/InventoryItems/PDA_InventoryItem` PDA_Ref)
    (:`then`
      (`self.Set Static Mesh and Scale` (`/Game/Dynamic/Code/Blueprints/BP_Pickups/PDA_Parent_Item.StaticMesh` _aspda_inventory_item) (`/Game/Dynamic/Code/Blueprints/BP_Pickups/PDA_Parent_Item.SpinScale` _aspda_inventory_item))
      ;[1 1 1] Changing the input control from the default to the itemspinner controls
      (`EnhancedInputSubsystemInterface.AddMappingContext` _returnvalue "/Game/Dynamic/Code/Blueprints/Inputs/IMC_ItemSpinner.IMC_ItemSpinner" 2 (struct) :!label _label)
      (`self.SetVisibility` true)
      (`EnhancedInputSubsystemInterface.RemoveMappingContext` _returnvalue "/Game/Dynamic/Code/Blueprints/Inputs/IMC_Default.IMC_Default" (struct)))
    (:`CastFailed`
      (bind _aspda_audio_item (cast `/Game/Dynamic/Code/Blueprints/BP_Pickups/AudioItems/PDA_AudioItem` PDA_Ref)
        (:`then`
          (`self.Set Static Mesh and Scale` (`/Game/Dynamic/Code/Blueprints/BP_Pickups/PDA_Parent_Item.StaticMesh` _aspda_audio_item) (`/Game/Dynamic/Code/Blueprints/BP_Pickups/PDA_Parent_Item.SpinScale` _aspda_audio_item))
          (goto _label))
        (:`CastFailed`
          (`KismetSystemLibrary.PrintString` "Bad Item"))))))

(event `EndSpin`
  (bind _returnvalue (pcsubsystem `EnhancedInputLocalPlayerSubsystem` (`self.Controller Ref`)))
  ;[1 1 1] Ending the 3d gimble view hiding the static mesh and setting it to be blank
  (`EnhancedInputSubsystemInterface.RemoveMappingContext` _returnvalue "/Game/Dynamic/Code/Blueprints/Inputs/IMC_ItemSpinner.IMC_ItemSpinner" (struct))
  (`self.SetVisibility` false)
  (`self.SetStaticMesh` null)
  (`EnhancedInputSubsystemInterface.AddMappingContext` _returnvalue "/Game/Dynamic/Code/Blueprints/Inputs/IMC_Default.IMC_Default" 0 (struct))
  (`self.K2_SetRelativeRotation` (struct)))

(fn `Set Static Mesh and Scale`
  (params (`Static Mesh` :type "StaticMesh Object Reference") (`3d scale` :type "Float (double-precision)"))
  (`self.SetStaticMesh` `Static Mesh`)
  (`self.SetRelativeScale3D` (`KismetMathLibrary.Conv_DoubleToVector` `3d scale`)))