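; Base pickup actor that tells overlapping actors when they can interact with it.
; Its Sphere component sends CanInteractMessage with true on begin overlap and false on end overlap, to any actor without filtering.
; The construction script sets the static mesh from a DataAsset, which GetDataAsset exposes to callers.
; The pickup or collection logic itself is not implemented here.
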(event `self.Sphere.OnComponentBeginOverlap`
  (params (OverlappedComponent :type "PrimitiveComponent Object Reference") (OtherActor :type "Actor Object Reference") (OtherComp :type "PrimitiveComponent Object Reference") (OtherBodyIndex :type Integer) (bFromSweep :type Boolean) (SweepResult :type "HitResult Structure (by ref)"))
  (message `/Game/Dynamic/Code/Blueprints/BP_Interfaces/BPI_Interactable.CanInteract?` OtherActor true))

(event `self.Sphere.OnComponentEndOverlap`
  (params (OverlappedComponent :type "PrimitiveComponent Object Reference") (OtherActor :type "Actor Object Reference") (OtherComp :type "PrimitiveComponent Object Reference") (OtherBodyIndex :type Integer))
  (message `/Game/Dynamic/Code/Blueprints/BP_Interfaces/BPI_Interactable.CanInteract?` OtherActor false))

(fn `GetDataAsset`
  (returns (DataAssetParent :type "/Game/Dynamic/Code/Blueprints/BP_Pickups/PDA_Parent_Item Object Reference"))
  (return (`self.DataAsset`)))

(fn `UserConstructionScript`
  (`StaticMeshComponent.SetStaticMesh` (`self.StaticMesh`) (`/Game/Dynamic/Code/Blueprints/BP_Pickups/PDA_Parent_Item.StaticMesh` (`self.DataAsset`))))