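; BP_Door is an interactable door that can be locked and opened with a matching inventory key data asset.
; Being looked at briefly enables its outline depth and sends the player an interaction message with the door's gameplay tag.
; OpenDoor checks the key, shows errors on failure, and returns true only when it unlocks.
; A FlipFlop alternates two timelines that incrementally nudge relative yaw to swing it open or closed.
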(event `/Game/Dynamic/Code/Blueprints/BP_Interfaces/BPI_Interactable.LookedAt`
  (params (PlayerCharacterRef :type "/Game/Dynamic/Code/Blueprints/Character/BP_FirstPersonCharacter Object Reference"))
  ;[1 1 1] Sends a message when object is being looked at. Sends gameplay tag as a door.
  (message `/Game/Dynamic/Code/Blueprints/BP_Interfaces/BPI_Interactable.CanInteract?` PlayerCharacterRef true (`self.GameplayTagType`))
  (`PrimitiveComponent.SetRenderCustomDepth` (`self.Door`) true)
  (`KismetSystemLibrary.RetriggerableDelay` 0.05)
  (message `/Game/Dynamic/Code/Blueprints/BP_Interfaces/BPI_Interactable.CanInteract?` PlayerCharacterRef false (struct))
  (`PrimitiveComponent.SetRenderCustomDepth` (`self.Door`) false))

(event `OpenDoorEvent`
  (bind (_relativerotation_roll _relativerotation_pitch _relativerotation_yaw) (`KismetMathLibrary.BreakRotator` (`SceneComponent.RelativeRotation` (`self.Door`))))
  (bind (_relativerotation_roll_2 _relativerotation_pitch_2 _relativerotation_yaw_2) (`KismetMathLibrary.BreakRotator` (`SceneComponent.RelativeRotation` (`self.Door`))))
  ;[1 1 1] Rotators the door open then rotatates the door closed.
  (`/Engine/EditorBlueprintResources/StandardMacros.FlipFlop`
    (:`A`
      (bind (_direction _opendoor) (`Timeline|DoorOpen` :!via `PlayFromStart`)
        (:`Update`
          (`SceneComponent.K2_SetRelativeRotation` (`self.Door`) (`KismetMathLibrary.MakeRotator` _relativerotation_roll_2 _relativerotation_pitch_2 (`KismetMathLibrary.Lerp` (+ _relativerotation_yaw_2 -1.5) _relativerotation_yaw_2 _opendoor)) false false))))
    (:`B`
      (bind (_direction_2 _opendoor_2) (`Timeline|Timeline` :!via `PlayFromStart`)
        (:`Update`
          (`SceneComponent.K2_SetRelativeRotation` (`self.Door`) (`KismetMathLibrary.MakeRotator` _relativerotation_roll _relativerotation_pitch (`KismetMathLibrary.Lerp` (+ _relativerotation_yaw 1.5) _relativerotation_yaw _opendoor_2)) false false))))))

(fn `GetDataAsset`
  (returns (DataAssetParent :type "/Game/Dynamic/Code/Blueprints/BP_Pickups/PDA_Parent_Item Object Reference"))
  (return null))

(fn `OpenDoor`
  (params (PDA_Key :type "/Game/Dynamic/Code/Blueprints/BP_Pickups/PDA_Parent_Item Object Reference"))
  (returns (`Success?` :type Boolean))
  (if (`self.DoorLocked?`)
    (bind _aspda_inventory_item (cast `/Game/Dynamic/Code/Blueprints/BP_Pickups/InventoryItems/PDA_InventoryItem` PDA_Key)
      (:`then`
        (if (== _aspda_inventory_item (`self.DA_Unlocker`))
          (set `self.DoorLocked?` false)
          (`self.OpenDoorEvent`)
          (return true)
          (else
            (message `/Game/Dynamic/Code/Blueprints/BP_Interfaces/BPI_Errors.ErrorMessage` (`GameplayStatics.GetPlayerCharacter` 0) "This is the wrong key")
            (return false))))
      (:`CastFailed`
        (message `/Game/Dynamic/Code/Blueprints/BP_Interfaces/BPI_Errors.ErrorMessage` (`GameplayStatics.GetPlayerCharacter` 0) "This Door is Locked you need a key")
        (return false)))
    (else
      (`self.OpenDoorEvent`)
      (return false))))

(fn `UserConstructionScript`)